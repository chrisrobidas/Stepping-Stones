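; Torch weapon Blueprint that burns for a set duration when triggered.
; Burn turns on actor collision and shows the Box component while Tick accumulates the burn time.
; When the duration elapses, it resets the timer, disables collision, hides the Box and notifies the owning Character that the attack has ended.
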(event `self.ReceiveBeginPlay`)

(event `self.ReceiveTick`
  (params (DeltaSeconds :type "Float (single-precision)"))
  (if (`self._isBurning`)
    (if (>= (`self._timeSinceStartOfBurning`) (`self._duration`))
      (set `self._isBurning` false)
      (set `self._timeSinceStartOfBurning` 0.0)
      (`self.SetActorEnableCollision` false)
      (`SceneComponent.SetHiddenInGame` (`self.Box`) true false)
      (`/Game/Player/BP_PlayerCharacter.AttackEnded` (`self._character`))
      (else
        (set `self._timeSinceStartOfBurning` (+ DeltaSeconds (`self._timeSinceStartOfBurning`)))))))

(event `Burn`
  (set `self._isBurning` true)
  (`self.SetActorEnableCollision` true)
  (`SceneComponent.SetHiddenInGame` (`self.Box`) false false))

(fn `UserConstructionScript`)