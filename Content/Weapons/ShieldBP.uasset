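; ShieldBP is a weapon Blueprint for a shield that performs a timed block.
; Block turns on actor collision, reveals the Box component and sets the blocking flag.
; While blocking, Tick accumulates elapsed time until it reaches BlockingDuration, then resets the timer, disables collision, hides the Box and calls AttackEnded on the owning Character.
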(event `self.ReceiveBeginPlay`)

(event `self.ReceiveTick`
  (params (DeltaSeconds :type "Float (single-precision)"))
  (if (`self._isBlocking`)
    (if (>= (`self._timeSinceStartOfBlocking`) (`self._blockingDuration`))
      (set `self._isBlocking` false)
      (set `self._timeSinceStartOfBlocking` 0.0)
      (`self.SetActorEnableCollision` false)
      (`SceneComponent.SetHiddenInGame` (`self.Box`) true false)
      (`/Game/Player/BP_PlayerCharacter.AttackEnded` (`self._character`))
      (else
        (set `self._timeSinceStartOfBlocking` (+ DeltaSeconds (`self._timeSinceStartOfBlocking`)))))))

(event `Block`
  (set `self._isBlocking` true)
  (`self.SetActorEnableCollision` true)
  (`SceneComponent.SetHiddenInGame` (`self.Box`) false false))

(fn `UserConstructionScript`)