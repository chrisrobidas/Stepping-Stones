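; Player character for Wukong in an obstacle game with movement locked to its starting Y, a time-based score and a pause menu toggle.
; BeginPlay spawns and attaches Torch and Shield actors and creates the HUD; key presses trigger burn or block, gated by possession and an attack lock.
; Obstacle hits knock the character back, briefly stun it and signal the big bad guy to close in.
; Wwise switches select footstep and landing sounds by ground type.
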(event `Key|Escape`
  (params (Key :type "Key Structure"))
  (:`Pressed`
    (if (`GameplayStatics.IsGamePaused`) :!label _label
      (`GameplayStatics.SetGamePaused` false)
      (`Widget.RemoveFromParent` (stale _returnvalue))
      (else
        (`GameplayStatics.SetGamePaused` true)
        (bind _returnvalue (`|CreateWidget` "/Game/UI/UI_DeathScreenNPause/W_Pause.W_Pause_C"))
        (`UserWidget.AddToViewport` _returnvalue 0)))))

(event `Key|P` :paused true
  (params (Key :type "Key Structure"))
  (:`Pressed`
    (goto _label)))

(event `AttackEnded`
  (`KismetSystemLibrary.Delay` 0.4)
  (set `self.isUsingAttack` false))

(event `Key|F`
  (params (Key :type "Key Structure"))
  (:`Pressed`
    (if (`self.hasTorch`)
      (if (not (`self.isUsingAttack`))
        (set `self.isUsingAttack` true)
        (`/Game/Weapons/TorchBP.Burn` (`self.Torch`) (`self.TorchMesh`))))))

(event `Key|D`
  (params (Key :type "Key Structure"))
  (:`Pressed`
    (if (`self.hasShield`)
      (if (not (`self.isUsingAttack`))
        (set `self.isUsingAttack` true)
        (`/Game/Weapons/ShieldBP.Block` (`self.Shield`) (`self.ShieldMesh`))))))

(event `self.ReceiveBeginPlay`
  (bind _location (.location (`self.GetTransform`)))
  (bind _rotation (.rotation (`self.GetTransform`)))
  (bind _scale (.scale (`self.GetTransform`)))
  (`|ExecutionSequence`
    (:`then_0`
      (bind _returnvalue (`|SpawnActorFromClass` "/Game/Weapons/TorchBP.TorchBP_C" (`KismetMathLibrary.MakeTransform` (+ (* (`self.GetActorForwardVector`) 80.0) _location) _rotation _scale) "AlwaysSpawn" "OverrideRootScale" null null))
      (bind _output_get (set `self.Torch` _returnvalue))
      (`self.K2_AttachToActor` _output_get self "Hand_Socket" "KeepWorld" "KeepRelative" "KeepRelative" true)
      (`self.SetActorEnableCollision` _output_get false)
      (set `/Game/Weapons/TorchBP._character` self _output_get)
      (`SceneComponent.SetVisibility` (`self.TorchMesh`) false true))
    (:`then_1`
      (bind _returnvalue_2 (`|SpawnActorFromClass` "/Game/Weapons/ShieldBP.ShieldBP_C" (`KismetMathLibrary.MakeTransform` (+ _location (* (`self.GetActorForwardVector`) 20.0) (* (`self.GetActorUpVector`) 90.0)) _rotation _scale) "AlwaysSpawn" "OverrideRootScale" null null))
      (bind _output_get_2 (set `self.Shield` _returnvalue_2))
      (`self.K2_AttachToActor` _output_get_2 self "Hand_Socket" "KeepWorld" "KeepRelative" "KeepRelative" true)
      (`self.SetActorEnableCollision` _output_get_2 false)
      (set `/Game/Weapons/ShieldBP._character` self _output_get_2)
      (`SceneComponent.SetVisibility` (`self.ShieldMesh`) false true))
    (:`then_2`
      (bind _returnvalue_3 (`|CreateWidget` "/Game/UI/UI_HUD/W_HUD.W_HUD_C"))
      (`UserWidget.AddToViewport` _returnvalue_3 0)
      (set `/Game/UI/UI_HUD/W_HUD._character` self _returnvalue_3)
      (set `self.HUD` _returnvalue_3))
    (:`then_3`
      (set `self.InitialYPosition` (`.Y` (`KismetMathLibrary.BreakVector3f` (`SceneComponent.K2_GetComponentLocation` (`self._capsule`))))))))

(event `self.ReceiveHit`
  (params (MyComp :type "PrimitiveComponent Object Reference") (Other :type "Actor Object Reference") (OtherComp :type "PrimitiveComponent Object Reference") (bSelfMoved :type Boolean) (HitLocation :type "Vector Structure") (HitNormal :type "Vector Structure") (NormalImpulse :type "Vector Structure") (Hit :type "HitResult Structure (by ref)"))
  (if (`self.ActorHasTag` Other "Obstacle")
    (`|ExecutionSequence`
      (:`then_0`
        (`self.BigBadGuyCloserDispatcher`)
        (`KismetSystemLibrary.MoveComponentTo` (`self.CapsuleComponent`) (+ (.location (`SceneComponent.K2_GetComponentToWorld` (`self.CapsuleComponent`))) (-500.0 0.0 0.0)) (struct) true false 0.7))
      (:`then_1`
        (set `self.isKnockOut` true)
        (`KismetSystemLibrary.Delay` 0.5)
        (set `self.isKnockOut` false)))))

(event `self.ReceiveTick`
  (params (DeltaSeconds :type "Float (single-precision)"))
  (bind __capsule (`self._capsule`))
  (bind _charactermovement (`self.CharacterMovement`))
  (bind (_x _y _z) (`KismetMathLibrary.BreakVector3f` (`SceneComponent.K2_GetComponentLocation` __capsule)))
  (`|ExecutionSequence`
    (:`then_0`
      (`KismetSystemLibrary.Delay` 0.5)
      (set `self.Score` (+ (`self.Score`) 1)))
    (:`then_1`
      ;[1 1 1] Locks character to it's initial Y location
      (`SceneComponent.K2_SetWorldLocation` __capsule (`KismetMathLibrary.MakeVector` _x (`self.InitialYPosition`) _z) false true))
    (:`then_2`
      ;[1 1 1] Footsteps sound when on ground and moving
      (if (and (not (`NavMovementComponent.IsFalling` _charactermovement)) (> (`KismetMathLibrary.VSize` (`MovementComponent.Velocity` _charactermovement)) 0.0))
        (`KismetSystemLibrary.Delay` 0.4)
        (`AkGameplayStatics.SetSwitch` null null "SW_Player_FT_Surfaces" (`KismetStringLibrary.Conv_StringToName` (`self.GroundType`)))
        (`AkGameplayStatics.PostEvent` "/Game/Audio/Play_Player_FT.Play_Player_FT" self)))))

(event `self.OnLanded`
  (params (Hit :type "HitResult Structure (by ref)"))
  ;[1 1 1] Land sound when landing
  (`AkGameplayStatics.SetSwitch` null null "SW_Player_Jump_Surfaces" (`KismetStringLibrary.Conv_StringToName` (`self.GroundType`)))
  (`AkGameplayStatics.PostEvent` "/Game/Audio/Play_Player_Jump_Surfaces_Land.Play_Player_Jump_Surfaces_Land" self))

(fn `UserConstructionScript`)