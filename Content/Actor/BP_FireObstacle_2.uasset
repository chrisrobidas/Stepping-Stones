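; Fire obstacle actor whose Cube gives way when overlapped by a TorchBP actor or when its Hit event fires.
; Both paths disable the Cube's collision, move and rotate it with MoveComponentTo, and set a lifespan so the actor destroys itself.
; The torch overlap uses a fixed, eased-in swing, while Hit uses a tumbling rotation timed by the DissapearingTime variable.
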(event `self.ReceiveActorBeginOverlap`
  (params (OtherActor :type "Actor Object Reference"))
  (bind _cube (`self.Cube`))
  (if (`GameplayStatics.ObjectIsA` OtherActor "/Game/Weapons/TorchBP.TorchBP_C")
    (`PrimitiveComponent.SetCollisionEnabled` _cube "NoCollision")
    (`self.SetLifeSpan` 1.0)
    (`KismetSystemLibrary.MoveComponentTo` _cube (100.0 0.0 0.0) (struct :`Pitch` -90.0) false true 0.6 true)))

(event `self.ReceiveHit`
  (params (MyComp :type "PrimitiveComponent Object Reference") (Other :type "Actor Object Reference") (OtherComp :type "PrimitiveComponent Object Reference") (bSelfMoved :type Boolean) (HitLocation :type "Vector Structure") (HitNormal :type "Vector Structure") (NormalImpulse :type "Vector Structure") (Hit :type "HitResult Structure (by ref)"))
  (bind _cube (`self.Cube`))
  (bind _dissapearingtime (`self.DissapearingTime`))
  (`PrimitiveComponent.SetCollisionEnabled` _cube "NoCollision")
  (`self.SetLifeSpan` _dissapearingtime)
  (`KismetSystemLibrary.MoveComponentTo` _cube (100.0 0.0 0.0) (struct :`Pitch` -75.0 :`Yaw` 75.0 :`Roll` 10.0) false false _dissapearingtime))

(fn `UserConstructionScript`)