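; BP_BigBadGuyV2 is an enemy actor that chases the player along the X axis and ends play on contact.
; Tick issues a slow timed MoveComponentTo on the root toward the player's X position, keeping its own Y and Z.
; Overlapping a PlayerCharacter pauses the game and adds the W_DeathScreen widget to the viewport.
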(event `self.ReceiveActorBeginOverlap`
  (params (OtherActor :type "Actor Object Reference"))
  (if (`KismetMathLibrary.ClassIsChildOf` (`GameplayStatics.GetObjectClass` OtherActor) "/Script/MTL_Game_Jam_2023.PlayerCharacter")
    (`GameplayStatics.SetGamePaused` true)
    (bind _returnvalue (`|CreateWidget` "/Game/UI/UI_DeathScreenNPause/W_DeathScreen.W_DeathScreen_C"))
    (`UserWidget.AddToViewport` _returnvalue 0)))

(event `self.ReceiveTick`
  (params (DeltaSeconds :type "Float (single-precision)"))
  (bind (_x _y _z) (`KismetMathLibrary.BreakVector3f` (`self.K2_GetActorLocation`)))
  (`KismetSystemLibrary.MoveComponentTo` (`self.RootComponent`) (`KismetMathLibrary.MakeVector` (`KismetMathLibrary.BreakVector3f` (`self.K2_GetActorLocation` (`GameplayStatics.GetPlayerCharacter` 0))) _y _z) (struct) false false 20.0))

(fn `UserConstructionScript`)