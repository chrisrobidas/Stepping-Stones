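; BP_BigBadGuy is a pursuing threat whose sphere trails the player at an offset and ends the game when it gets too close.
; The offset starts at the sphere's world location, then shifts periodically through a Tick-driven Delay and whenever BP_WukongCharacter's closer dispatcher fires.
; Tick eases the sphere toward player location plus offset.
; Once the offset's X exceeds DeathDistance, it pauses and shows W_DeathScreen.
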(event `self.ReceiveTick`
  (params (DeltaSeconds :type "Float (single-precision)"))
  (`|ExecutionSequence`
    (:`then_0`
      (`KismetSystemLibrary.Delay` DeltaSeconds)
      (`KismetSystemLibrary.MoveComponentTo` (`self.Sphere`) (+ (`self.K2_GetActorLocation` (`GameplayStatics.GetPlayerCharacter` 0)) (stale _output_get)) (struct) true true DeltaSeconds)
      (`/Engine/EditorBlueprintResources/StandardMacros.CompareFloat` (.x (stale _output_get)) (`self.DeathDistance`)
        (:`>`
          (`GameplayStatics.SetGamePaused` true)
          (bind _returnvalue (`|CreateWidget` "/Game/UI/UI_DeathScreenNPause/W_DeathScreen.W_DeathScreen_C"))
          (`UserWidget.AddToViewport` _returnvalue 0))))
    (:`then_1`
      (`KismetSystemLibrary.Delay` (`self.DeathTimerTime`))
      (bind _output_get (set `self.DistanceVector` (+ (`self.DistanceVector`) (`self.DeathTimerValue`)))))))

(event `self.ReceiveBeginPlay`
  (`|ExecutionSequence`
    (:`then_0`
      (bind _asbp_player_character (cast `/Game/Player/BP_WukongCharacter` (`GameplayStatics.GetPlayerCharacter` 0)))
      (add `/Game/Player/BP_WukongCharacter.BigBadGuyCloserDispatcher` _asbp_player_character (delegate `BigBadGuyGetCloser`)))
    (:`then_1`
      (set `self.DistanceVector` (`SceneComponent.K2_GetComponentLocation` (`self.Sphere`))))))

(event `BigBadGuyGetCloser`
  (set `self.DistanceVector` (+ (`self.DistanceVector`) (`self.HitDistance`))))

(fn `UserConstructionScript`)